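; ChainsawKid_BP is the playable chainsaw kid, with lane-based steering, a pause action and a configurable spring arm camera.
; Steer axis input is forwarded to the ACOLaneShifting component.
; Pause freezes the game, opens a new PauseMenu_W, shows the cursor and switches input to UI only.
; The construction script sets the spring arm's world rotation from negated camera angle variables, along with its length.
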(event `self.ReceiveBeginPlay`
  (`KismetSystemLibrary.PrintString` "chainsaw kid created"))

(event `InputAxis|Steer`
  (params (AxisValue :type "Float (single-precision)"))
  (`/Game/Character/Chainsaw/ACO_LaneShifting.LaneSteer` (`self.ACO_LaneShifting`) AxisValue))

(event `InputAction|Pause`
  (params (Key :type "Key Structure"))
  (bind _returnvalue (`GameplayStatics.GetPlayerController` 0))
  (:`Pressed`
    (`GameplayStatics.SetGamePaused` true)
    (bind _returnvalue_2 (`|CreateWidget` "/Game/Widget/PauseMenu_W.PauseMenu_W_C"))
    (`UserWidget.AddToViewport` _returnvalue_2 0)
    (set `PlayerController.bShowMouseCursor` true _returnvalue)
    (`WidgetBlueprintLibrary.SetInputMode_UIOnlyEx` _returnvalue _returnvalue_2)))

(fn `UserConstructionScript`
  (`SceneComponent.K2_SetWorldRotation` (`self.SpringArm`) (`KismetMathLibrary.MakeRotator` 0.0 (`KismetMathLibrary.Conv_IntToDouble` (* (`self.CameraYAngle`) -1)) (`KismetMathLibrary.Conv_IntToDouble` (* (`self.CameraZAngle`) -1))) false false)
  (set `SpringArmComponent.TargetArmLength` (`self.SpringArmLength`) (`self.SpringArm`)))